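; BP_Pendulum is a pendulum actor that rotates its Pivot component in pitch.
; BeginPlay calls PendulumTimer once, which adds RotationValue as local pitch; no timer or loop here repeats it.
; If world pitch reaches Angle, the function snaps to that pitch with zero roll and yaw, then steps back by RotationValue.
; The Hit event is empty and the Frequency variable is unused.
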(event Collision|EventHit
  (params (MyComp :type Primitive%20Component%20Object%20Reference) (Other :type Actor%20Object%20Reference) (OtherComp :type Primitive%20Component%20Object%20Reference) (bSelfMoved :type Boolean) (HitLocation :type Vector :default "0, 0, 0") (HitNormal :type Vector :default "0, 0, 0") (NormalImpulse :type Vector :default "0, 0, 0") (Hit :type Hit%20Result%20Structure%20%28by%20ref%29)))

(event EventBeginPlay
  (CallFunction|PendulumTimer))

(fn ConstructionScript)

(fn PendulumTimer
  (bind _pivot (Variables|Default|GetPivot))
  (bind _angle (Variables|Default|GetAngle))
  (Transformation|AddLocalRotation _pivot (Math|Rotator|MakeRotator 0.0 (Variables|Default|GetRotationValue) 0.0) false false)
  (if (>= (.pitch (Transformation|GetWorldRotation _pivot)) _angle)
    (Transformation|SetWorldRotation (Variables|Default|GetPivot) (Math|Rotator|MakeRotator 0.0 _angle 0.0) false false)
    (Transformation|AddLocalRotation (Variables|Default|GetPivot) (Math|Rotator|MakeRotator 0.0 (* -1 (Variables|Default|GetRotationValue)) 0.0) false false)))